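; Base enemy actor, named as a parent class, that drops in on spawn and then travels sideways along world X.
; BeginPlay picks a random direction and speed, increments the enemy count in BP_DanGameMode, and plays a timeline lowering it 120 units.
; When the timeline finishes, Tick starts moving it without sweep, adding DeltaSeconds to the step rather than scaling by it, so speed is frame-rate dependent.
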(event `self.ReceiveBeginPlay`
  (bind _spawnlocation (`self.SpawnLocation`))
  ;[1 1 1] setup ref and var
  (`|ExecutionSequence`
    (:`then_0`
      (set `self.MoveDirection` (`KismetMathLibrary.RandomBool`)))
    (:`then_1`
      (bind _asbp_dan_game_mode (cast `/Game/Blueprints/BP_DanGameMode` (`GameplayStatics.GetGameMode`)))
      (bind _output_get (set `self.BP_DanGameMode` _asbp_dan_game_mode))
      (`/Game/Blueprints/BP_DanGameMode.UpdateEnemyCount` _output_get 1))
    (:`then_2`
      (set `self.MovementSpeed` (`KismetMathLibrary.RandomFloatInRange` (`self.MinSpeed`) (`self.MaxSpeed`))))
    (:`then_3`
      (set `self.SpawnLocation` (`self.K2_GetActorLocation`)))
    (:`then_4`
      ;[1 1 1] Spawn Animation
      (bind (_direction _entryspeed) (`Timeline|SpawnAnimation`)
        (:`Update`
          (`self.K2_SetActorLocation` (`KismetMathLibrary.VLerp` _spawnlocation (- _spawnlocation (0.0 0.0 120.0)) _entryspeed)))
        (:`Finished`
          (set `self.MoveEnabled` true))))))

(event `self.ReceiveTick`
  (params (DeltaSeconds :type "Float (single-precision)"))
  (if (`self.MoveEnabled`)
    (`self.K2_SetActorLocation` (+ (`self.K2_GetActorLocation`) (+ (`KismetMathLibrary.MakeVector` (* (`self.MovementSpeed`) (`KismetMathLibrary.SelectFloat` 1.0 -1.0 (`self.MoveDirection`)))) DeltaSeconds)))))

(fn `UserConstructionScript`)