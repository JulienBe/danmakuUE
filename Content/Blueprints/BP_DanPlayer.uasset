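; Player actor for the Dan game mode, moved on a vertical X-Z plane with smoothed axis input.
; On BeginPlay it caches the game mode and plays a timeline that raises and spins it, then sets MoveEnabled, which nothing here reads.
; The Movement function eases each axis speed toward its input target.
; Tick applies those speeds as a swept per-frame offset and turns yaw against horizontal speed.
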(event `self.ReceiveBeginPlay`
  (bind _spawnlocation (`self.SpawnLocation`))
  ;[1 1 1] Player Spawn Animation and init
  (bind _asbp_dan_game_mode (cast `/Game/Blueprints/BP_DanGameMode` (`GameplayStatics.GetGameMode`)))
  (set `self.BP_GameMode` _asbp_dan_game_mode)
  (set `self.Yaw` (.yaw (`self.K2_GetActorRotation`)))
  (set `self.SpawnLocation` (`self.K2_GetActorLocation`))
  (bind (_direction _speed) (`Timeline|SpawnAnimation`)
    (:`Update`
      (`self.K2_SetActorLocation` (`KismetMathLibrary.VLerp` _spawnlocation (+ _spawnlocation (0.0 0.0 60.0)) _speed))
      (`self.K2_SetActorRotation` (`KismetMathLibrary.RLerp` (struct) (`KismetMathLibrary.MakeRotator` 0.0 0.0 (+ (`self.Yaw`) (`self.Spawn Spin Count`))) _speed)))
    (:`Finished`
      (set `self.MoveEnabled` true))))

(event `self.ReceiveTick`
  (params (DeltaSeconds :type "Float (single-precision)"))
  ;[1 1 1] Input
  (set `self.Delta` DeltaSeconds)
  (`|ExecutionSequence`
    (:`then_0`
      (`self.K2_SetActorLocation` (+ (`self.K2_GetActorLocation`) (`KismetMathLibrary.MakeVector` (`self.HorizontalSpeed`) 0.0 (`self.VerticalSpeed`))) true))
    (:`then_1`
      (`self.K2_SetActorRotation` (`KismetMathLibrary.RInterpTo_Constant` (`self.K2_GetActorRotation`) (`KismetMathLibrary.MakeRotator` 0.0 0.0 (+ (* (`self.HorizontalSpeed`) -15.0) (`self.Yaw`))) (`self.Delta`) (`self.YawInterpSpeed`))))))

(event `InputAxis|MovementX`
  (params (AxisValue :type "Float (single-precision)"))
  ;[1 1 1] Movement
  (bind _dirspeed (`self.Movement` (`self.HorizontalSpeed`) AxisValue))
  (set `self.HorizontalSpeed` _dirspeed))

(event `InputAxis|MovementY`
  (params (AxisValue :type "Float (single-precision)"))
  ;[1 1 1] Movement
  (bind _dirspeed (`self.Movement` (`self.VerticalSpeed`) AxisValue))
  (set `self.VerticalSpeed` _dirspeed))

(fn `Movement`
  (params (CurrentSpeed :type "Float (double-precision)") (Direction :type "Float (double-precision)"))
  (returns (DirSpeed :type "Float (double-precision)"))
  (return (`KismetMathLibrary.FInterpTo` CurrentSpeed (* Direction (`self.MovementSpeed`)) (`self.Delta`) (`self.InterpSpeed`))))

(fn `UserConstructionScript`)