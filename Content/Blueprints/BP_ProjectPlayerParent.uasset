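; Parent projectile Blueprint, apparently for player shots, exposing scale, speed and color.
; Its construction script uses a non-looping MultiGate, which fires one output per execution, to route mesh scaling, ProjectileMovement speed setup and dynamic material creation.
; BeginPlay clears the ProjectileMaterial reference before setting its Color parameter, so that color call has no material to act on.
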(event `self.ReceiveBeginPlay`
  (bind _output_get (set `self.ProjectileMaterial` null))
  (`MaterialInstanceDynamic.SetVectorParameterValue` _output_get "Color" (`self.ProjectileColor`)))

(fn `UserConstructionScript`
  (bind _projectilemovement (`self.ProjectileMovement`))
  (bind _speed (`self.Speed`))
  (`|MultiGate` false
    (:`Out 0`
      (`SceneComponent.SetWorldScale3D` (`self.Projectile`) (`self.Scale`)))
    (:`Out 1`
      (set `ProjectileMovementComponent.MaxSpeed` _speed _projectilemovement))
    (:`Out 2`
      (set `ProjectileMovementComponent.InitialSpeed` _speed _projectilemovement))
    (:`Out 3`
      (bind _returnvalue (`PrimitiveComponent.CreateDynamicMaterialInstance` (`self.Projectile`) 0 null))
      (set `self.ProjectileMaterial` _returnvalue))))